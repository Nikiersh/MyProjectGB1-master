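; AMMO_AC is an ammo counter, apparently an Actor Component, that tracks the current ammo of its owner.
; It fills current ammo to MaxAmmo on BeginPlay.
; SubstructAmmo deducts a given amount, clamped between zero and the maximum, and CheckAmmo reports whether enough remains for a given cost.
; It has no reload or refill logic, and Tick is unused.
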(event `self.ReceiveBeginPlay`
  (set `self.Сurrent Ammo` (`self.Max Ammo`)))

(fn `Check Ammo`
  (params (Value :type Integer))
  (returns (ReturnValue :type Boolean))
  (return (>= (`self.Сurrent Ammo`) Value)))

(fn `Substruct Ammo`
  (params (Value :type Integer :default 1))
  (set `self.Сurrent Ammo` (`KismetMathLibrary.Clamp` (- (`self.Сurrent Ammo`) Value) 0 (`self.Max Ammo`))))