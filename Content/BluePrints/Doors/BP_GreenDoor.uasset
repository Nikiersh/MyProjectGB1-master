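; BP_GreenDoor is a rotating door that the player opens and closes with the Interact input while holding the green key.
; Its Boxdoor overlap events enable and disable input, and the press checks HasGreenKey on BP_UnderScore_TopDown_Char and the GreenDoorTime flag.
; GreenDoorOpen then selects playing or reversing a Timeline that yaws the door up to 90 degrees and updates that flag from its track value.
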(event `self.boxdoor.OnComponentBeginOverlap`
  (params (OverlappedComponent :type "PrimitiveComponent Object Reference") (OtherActor :type "Actor Object Reference") (OtherComp :type "PrimitiveComponent Object Reference") (OtherBodyIndex :type Integer) (bFromSweep :type Boolean) (SweepResult :type "HitResult Structure (by ref)"))
  (`self.EnableInput` (`GameplayStatics.GetPlayerController` 0))
  (bind _asbp_under_score_top_down_char (cast `/Game/character/BP_UnderScore_TopDown_Char` (`GameplayStatics.GetPlayerCharacter` 0)))
  (if (`/Game/character/BP_UnderScore_TopDown_Char.HasGreenKey` _asbp_under_score_top_down_char)
    _))

(event `self.boxdoor.OnComponentEndOverlap`
  (params (OverlappedComponent :type "PrimitiveComponent Object Reference") (OtherActor :type "Actor Object Reference") (OtherComp :type "PrimitiveComponent Object Reference") (OtherBodyIndex :type Integer))
  (`self.DisableInput` (`GameplayStatics.GetPlayerController` 0)))

(event `InputAction|Interact`
  (params (Key :type "Key Structure"))
  (:`Pressed`
    (bind _asbp_under_score_top_down_char (cast `/Game/character/BP_UnderScore_TopDown_Char` (`GameplayStatics.GetPlayerCharacter` 0)))
    (if (`/Game/character/BP_UnderScore_TopDown_Char.HasGreenKey` _asbp_under_score_top_down_char)
      (if (`self.GreenDoorTime`)
        (if (`self.GreenDoorOpen`)
          (set `self.GreenDoorOpen` false)
          (bind (_direction _newtrack_0) (`Timeline|Timeline` :!label _label)
            (:`Update`
              (`SceneComponent.K2_SetRelativeRotation` (`self.door`) (`KismetMathLibrary.MakeRotator` 0.0 0.0 (* _newtrack_0 90.0)) false false)
              (set `self.GreenDoorOpen` (not (> _newtrack_0 0.0))))
            (:`Finished`
              (set `self.GreenDoorOpen` false)))
          (else
            (set `self.GreenDoorOpen` false)
            (goto _label :!via `ReverseFromEnd`)))))))

(fn `UserConstructionScript`)