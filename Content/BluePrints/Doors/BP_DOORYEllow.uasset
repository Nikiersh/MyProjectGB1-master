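; Yellow door actor that the player opens and closes with Interact while holding the yellow key.
; The box overlap toggles input and shows the NeedAYellowKey component whether or not the key is held, turning it toward the player only with the key.
; Interact checks the key and Doortime, then plays or reverses a timeline based on Dooropen.
; The mesh yaw and Dooropen are set from the timeline track on its Finished output.
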(event `self.Box.OnComponentBeginOverlap`
  (params (OverlappedComponent :type "PrimitiveComponent Object Reference") (OtherActor :type "Actor Object Reference") (OtherComp :type "PrimitiveComponent Object Reference") (OtherBodyIndex :type Integer) (bFromSweep :type Boolean) (SweepResult :type "HitResult Structure (by ref)"))
  (bind _need_a_yellow_key (`self.need a yellow key`))
  (`self.EnableInput` (`GameplayStatics.GetPlayerController` 0))
  (bind _asbp_under_score_top_down_char (cast `/Game/character/BP_UnderScore_TopDown_Char` (`GameplayStatics.GetPlayerCharacter` 0)))
  (if (`/Game/character/BP_UnderScore_TopDown_Char.HasYelloyKey` _asbp_under_score_top_down_char)
    (`SceneComponent.SetVisibility` _need_a_yellow_key true false)
    (`SceneComponent.K2_SetRelativeRotation` _need_a_yellow_key (`KismetMathLibrary.FindLookAtRotation` (`self.K2_GetActorLocation`) (`self.K2_GetActorLocation` (`GameplayStatics.GetPlayerCharacter` 0))) false false)
    (else
      (`SceneComponent.SetVisibility` (`self.need a yellow key`) true false))))

(event `self.Box.OnComponentEndOverlap`
  (params (OverlappedComponent :type "PrimitiveComponent Object Reference") (OtherActor :type "Actor Object Reference") (OtherComp :type "PrimitiveComponent Object Reference") (OtherBodyIndex :type Integer))
  (`self.DisableInput` (`GameplayStatics.GetPlayerController` 0)))

(event `InputAction|Interact`
  (params (Key :type "Key Structure"))
  (:`Pressed`
    (bind _asbp_under_score_top_down_char (cast `/Game/character/BP_UnderScore_TopDown_Char` (`GameplayStatics.GetPlayerCharacter` 0)))
    (if (`/Game/character/BP_UnderScore_TopDown_Char.HasYelloyKey` _asbp_under_score_top_down_char)
      (if (`self.doortime`)
        (if (`self.dooropen`)
          (set `self.dooropen` false)
          (bind (_direction _newtrack_0) (`Timeline|Timeline` :!label _label)
            (:`Finished`
              (set `self.dooropen` false)
              (`SceneComponent.K2_SetRelativeRotation` (`self.StaticMesh`) (`KismetMathLibrary.MakeRotator` 0.0 0.0 (* _newtrack_0 90.0)) false false)
              (set `self.dooropen` (not (> _newtrack_0 0.0)))))
          (else
            (set `self.dooropen` false)
            (goto _label :!via `ReverseFromEnd`)))))))

(fn `UserConstructionScript`)